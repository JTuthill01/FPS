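; Rifle weapon Blueprint that adds rifle-specific animation and effects to the fire and reload events of its parent weapon class.
; WeaponFire calls the parent logic, plays the rifle fire animation on WeaponMesh and spawns a shell-ejection particle at the AmmoEject socket.
; WeaponReload calls the parent logic, then plays the rifle reload animation on the same mesh.
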(event `self.WeaponFire`
  (bind (_returnvalue_location _returnvalue_rotation) (`KismetMathLibrary.BreakTransform` (`SceneComponent.GetSocketTransform` (`self.Weapon Mesh`) "AmmoEject" "RTS_World")))
  (`parent.WeaponFire`)
  (`SkeletalMeshComponent.PlayAnimation` (`self.Weapon Mesh`) "/Game/MilitaryWeapDark/Weapons/Anims/Fire_Rifle_W.Fire_Rifle_W" false)
  (`GameplayStatics.SpawnEmitterAtLocation` "/Game/Particles/FX_Rifle_Shells.FX_Rifle_Shells" _returnvalue_location _returnvalue_rotation))

(event `self.WeaponReload`
  (`parent.WeaponReload`)
  (`SkeletalMeshComponent.PlayAnimation` (`self.Weapon Mesh`) "/Game/Animations/FPP_Animations/FPP_RifleReload.FPP_RifleReload" false))

(fn `UserConstructionScript`
  (`parent.UserConstructionScript`))