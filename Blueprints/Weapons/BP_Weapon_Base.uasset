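; Base weapon Blueprint for an FPS, handling firing, hitscan shot calculation and magazine ammo for the player character cached at BeginPlay.
; WeaponFire decrements ammo, traces against world objects from the player camera with random endpoint spread, and spawns an impact actor from the result.
; The muzzle socket is stored but unused in the trace.
; Reload refills the magazine, but its reserve calculation and HasExtraAmmo read magazine ammo rather than the reserve.
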(event `self.ReceiveBeginPlay`
  (bind _asbp_fps_character (cast `/Game/Blueprints/BP_FPS_Character` (`GameplayStatics.GetPlayerPawn` 0)))
  (set `self.Player Ref` _asbp_fps_character))

(fn `CalcShot`
  (params (Camera :type "CameraComponent Object Reference") (WeaponMesh :type "SceneComponent Object Reference") (WeaponFireSocketName :type Name))
  (returns (HirResult :type "HitResult Structure"))
  (locals (LocalCamera :type "CameraComponent Object Reference") (LocalWeaponMesh :type "SceneComponent Object Reference") (SocketName :type "SceneComponent Object Reference") (LocalFireSocketName :type Name))
  (bind _bulletspread (`self.BulletSpread`))
  (bind (_returnvalue_location _returnvalue_rotation) (`KismetMathLibrary.BreakTransform` (`SceneComponent.K2_GetComponentToWorld` (`local.LocalCamera`))))
  (bind _returnvalue (* _bulletspread -1.0))
  (`|ExecutionSequence`
    (:`then_0`
      (set `local.LocalCamera` Camera)
      (set `local.LocalWeaponMesh` WeaponMesh)
      (set `local.LocalFireSocketName` WeaponFireSocketName))
    (:`then_1`
      (bind _outhit (`KismetSystemLibrary.LineTraceSingleForObjects` _returnvalue_location (`KismetMathLibrary.MakeVector` (+ (.x (+ _returnvalue_location (* (`KismetMathLibrary.GetForwardVector` _returnvalue_rotation) 10000.0))) (`KismetMathLibrary.RandomFloatInRange` _returnvalue _bulletspread)) (+ (.y (+ _returnvalue_location (* (`KismetMathLibrary.GetForwardVector` _returnvalue_rotation) 10000.0))) (`KismetMathLibrary.RandomFloatInRange` _returnvalue _bulletspread)) (+ (.z (+ _returnvalue_location (* (`KismetMathLibrary.GetForwardVector` _returnvalue_rotation) 10000.0))) (`KismetMathLibrary.RandomFloatInRange` _returnvalue _bulletspread))) (`|MakeArray` "ObjectTypeQuery1" "ObjectTypeQuery2" :!type "EObjectTypeQuery Enum") false (`|MakeArray` (`GameplayStatics.GetPlayerPawn` 0) :!type "Actor Object Reference")))
      (return _outhit))))

(fn `HasAmmoInMag`
  (returns (HasAmmo :type Boolean) (IsMagFull :type Boolean))
  (return (> (`self.CurrentAmmo`) 0) (== (`self.CurrentAmmo`) (`self.MaxMagAmmo`))))

(fn `HasExtraAmmo`
  (returns (`Has Extra Ammo` :type Boolean))
  (return (> (`self.CurrentAmmo`) 0)))

(fn `UserConstructionScript`)

(fn `WeaponFire`
  (set `self.CurrentAmmo` (- (`self.CurrentAmmo`) 1))
  (bind _hirresult (`self.CalcShot` (`/Game/Blueprints/BP_FPS_Character.Camera` (`self.Player Ref`)) (`self.Weapon Mesh`) "MuzzleFlash"))
  (bind (_bblockinghit _binitialoverlap _time _distance _location _impactpoint) (`GameplayStatics.BreakHitResult` _hirresult))
  (`|SpawnActorFromClass` (`self.ImpactAssetClass`) (`KismetMathLibrary.MakeTransform` _impactpoint) "Undefined" "OverrideRootScale" null _hirresult _bblockinghit null))

(fn `WeaponReload`
  (bind _returnvalue (`KismetMathLibrary.Min` (`self.MaxMagAmmo`) (`self.MaxMagAmmo`)))
  (set `self.CurrentAmmo` _returnvalue)
  (set `self.CurrentTotallAmmo` (- (`self.CurrentAmmo`) _returnvalue)))